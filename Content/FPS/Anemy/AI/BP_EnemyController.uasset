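; BP_EnemyController is the AI controller for enemies, setting up and starting their behavior logic on BeginPlay.
; It loads the BP_EnemyBB blackboard and seeds it with the pawn's spawn location as home, an idle time, and a random navigable point near the pawn as the first target.
; It then runs the BP_EnemyBT behavior tree, which takes over from there.
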(event EventBeginPlay
  (bind _returnvalue (Pawn|GetControlledPawn))
  (bind _returnvalue_2 (Transformation|GetActorLocation _returnvalue))
  ;[1 1 1] AI Behavior Logic Start / BeginPlay
  (Utilities|FlowControl|Sequence
    (:then_0
      (Class|AIController|UseBlackboard "/Game/FPS/Anemy/AI/BP_EnemyBB.BP_EnemyBB")
      (AI|Components|Blackboard|SetValueasVector (Variables|Default|GetBlackboard) (Variables|Default|GetHomeLocKey) _returnvalue_2)
      (AI|Components|Blackboard|SetValueasFloat (Variables|Default|GetBlackboard) (Variables|Default|GetIdleTimeKey) 2.0)
      (AI|Components|Blackboard|SetValueasVector (Variables|Default|GetBlackboard) (Variables|Default|GetTargetLocKey) (.RandomLocation (Class|NavigationSystemV1|GetRandomPointinNavigableRadius _returnvalue_2 5e+02 0 0))))
    (:then_1
      (AI|RunBehaviorTree "/Game/FPS/Anemy/AI/BP_EnemyBT.BP_EnemyBT"))))

(fn ConstructionScript)