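; BP_Enemy is an enemy character driven by a PEACE, CHASE, ATTACK and DEAD state machine.
; PawnSensing switches PEACE to CHASE when it sees a pawn.
; SetState mirrors the state to the AI Blackboard and sets walk speed, locking once DEAD.
; Damage reduces HP; at zero the enemy dies, calls DeadCheck on the Maw actor and raises the player's kill count and capped super gauge.
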(event OnSeePawn(PawnSensing)
  (params (Pawn :type Pawn%20Object%20Reference))
  ;[1 1 1] If Find Player -> CHASE State
  (if (Utilities|Enum|Equal(Enum) (Variables|Default|GetCurrentStatePawn) "NewEnumerator0")
    (Variables|Actor|SetInstigator Pawn)
    (CallFunction|SetState "NewEnumerator1")))

(event EventBeginPlay
  ;[1 1 1] Start State -> PEACE / BeginPlay
  (Variables|Default|SetCurrentHP (Variables|Default|GetMaxHP))
  (CallFunction|SetState "NewEnumerator0"))

(event Game|Damage|EventAnyDamage
  (params (Damage :type Float%20%28single-precision%29) (DamageType :type Damage%20Type%20Object%20Reference) (InstigatedBy :type Controller%20Object%20Reference) (DamageCauser :type Actor%20Object%20Reference))
  ;[1 1 1] Recive Damage
  (bind _output_get (Variables|Default|SetCurrentHP (- (Variables|Default|GetCurrentHP) Damage)))
  (if (not (> _output_get 0.0))
    (CallFunction|SetState "NewEnumerator3")
    ;;[1 0.3422 0.2122] If Anemy DEAD State -> Check Clear Condition
    (bind _outactors (Actor|GetAllActorsOfClass "/Game/FPS/Anemy/Maw.Maw_C"))
    (Default|DeadCheck (Utilities|Array|Get(acopy) _outactors))
    ;[1 1 1] Functional Option (Not Used)
    ;;[1 1 1] 킬 카운트 함수
    (Variables|Default|SetCurrentHP 0.0)
    (bind _asthird_person_character (Utilities|Casting|CastToThirdPersonCharacter (Game|GetPlayerCharacter 0)))
    (Variables|/Game/FPS/Charactor/ThirdPersonCharacter.ThirdPersonCharacter_C|SetKillCount _asthird_person_character (+ (Variables|/Game/FPS/Charactor/ThirdPersonCharacter.ThirdPersonCharacter_C|GetKillCount _asthird_person_character) 1.0))
    ;;[1 1 1] 필살기게이지 채우기 최대25임
    (bind _asthird_person_character_2 (Utilities|Casting|CastToThirdPersonCharacter (Game|GetPlayerCharacter 0)))
    ;;;[0.8777 0.1615 1] 필살게이지 25면 제자리
    (if (>= (Variables|/Game/FPS/Charactor/ThirdPersonCharacter.ThirdPersonCharacter_C|GetsuperGauge _asthird_person_character_2) 25.0)
      (Variables|/Game/FPS/Charactor/ThirdPersonCharacter.ThirdPersonCharacter_C|SetsuperGauge _asthird_person_character_2 (Variables|/Game/FPS/Charactor/ThirdPersonCharacter.ThirdPersonCharacter_C|GetMaxsuperGauge _asthird_person_character_2))
      (else
        ;;;[1 0.2176 0.2574] 한대 때리면 1씩 증가
        (Variables|/Game/FPS/Charactor/ThirdPersonCharacter.ThirdPersonCharacter_C|SetsuperGauge _asthird_person_character_2 (+ (Variables|/Game/FPS/Charactor/ThirdPersonCharacter.ThirdPersonCharacter_C|GetsuperGauge _asthird_person_character_2) 1.0))))))

(fn ConstructionScript)

(fn SetState
  (params (NewState :type BPE_EnemyState%20Enum :default "NewEnumerator0"))
  (bind _charactermovement (Variables|Character|GetCharacterMovement))
  (if (Utilities|Enum|NotEqual(Enum) (Variables|Default|GetCurrentStatePawn) "NewEnumerator3")
    (bind _output_get (Variables|Default|SetCurrentStatePawn NewState))
    (Utilities|FlowControl|Sequence
      (:then_0
        (AI|Components|Blackboard|SetValueasEnum (AI|GetBlackboard (Pawn|GetController)) (Variables|Default|GetStateKey) _output_get))
      (:then_1
        (switch Utilities|FlowControl|Switch|SwitchonBPE_EnemyState (Variables|Default|GetCurrentStatePawn)
          (:NewEnumerator0
            (Variables|/Script/Engine.CharacterMovementComponent|SetMaxWalkSpeed _charactermovement 3e+02))
          (:NewEnumerator1
            (Variables|/Script/Engine.CharacterMovementComponent|SetMaxWalkSpeed _charactermovement 6e+02))
          (:NewEnumerator2
            (Variables|/Script/Engine.CharacterMovementComponent|SetMaxWalkSpeed _charactermovement 6e+02 :!label _label))
          (:NewEnumerator3
            (goto _label)))))))