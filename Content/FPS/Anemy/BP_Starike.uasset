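; BP_Starike is an FPS enemy with a melee attack and difficulty-scaled stats.
; On BeginPlay it reads the GameSaveData game instance and, when OpenLevel is set, sets HP and attack power from the Easy, Normal, Hard or Hell flag.
; OnAttackBegin runs a short forward sphere trace against Pawn objects and applies the Attack value as damage to the hit actor.
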(event Custom|OnAttackBegin
  (bind _returnvalue (Transformation|GetActorLocation))
  ;[1 1 1] Attack
  (bind _outhit (Collision|SphereTraceForObjects _returnvalue (+ (* (Transformation|GetActorForwardVector) 1.5e+02) _returnvalue) 5e+01 (Utilities|Array|MakeArray "ObjectTypeQuery3") false 0 "None"))
  (Game|Damage|ApplyDamage (.HitActor (Collision|BreakHitResult _outhit)) (Variables|Default|GetAttack) 0 0))

(event EventBeginPlay
  ;[1 1 1] Begin Play
  (bind _asgame_save_data (Utilities|Casting|CastToGameSaveData (Game|GetGameInstance)))
  (if (Variables|/Game/FPS/GameSaveData.GameSaveData_C|GetOpenLevel _asgame_save_data)
    (Utilities|FlowControl|Sequence
      (:then_0
        (if (Variables|/Game/FPS/GameSaveData.GameSaveData_C|GetSetEasy _asgame_save_data)
          (bind _output_get (Variables|Default|SetMaxHP 3e+02))
          (Variables|Default|SetCurrentHP _output_get)
          (Variables|Default|SetAttack 4e+01)))
      (:then_1
        (if (Variables|/Game/FPS/GameSaveData.GameSaveData_C|GetSetNormal _asgame_save_data)
          (bind _output_get_2 (Variables|Default|SetMaxHP 6e+02))
          (Variables|Default|SetCurrentHP _output_get_2)
          (Variables|Default|SetAttack 5e+01)))
      (:then_2
        (if (Variables|/Game/FPS/GameSaveData.GameSaveData_C|GetSetHard _asgame_save_data)
          (bind _output_get_3 (Variables|Default|SetMaxHP 1.2e+03))
          (Variables|Default|SetCurrentHP _output_get_3)
          (Variables|Default|SetAttack 6e+01)))
      (:then_3
        (if (Variables|/Game/FPS/GameSaveData.GameSaveData_C|GetSetHell _asgame_save_data)
          (bind _output_get_4 (Variables|Default|SetMaxHP 3e+03))
          (Variables|Default|SetCurrentHP _output_get_4)
          (Variables|Default|SetAttack 8e+01))))))

(fn ConstructionScript
  (|CallParentFunction))